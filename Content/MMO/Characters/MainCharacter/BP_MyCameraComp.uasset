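; Camera component for the MMO main character that switches its parent spring arm between default, melee, range and aim framing.
; BeginPlay caches the parent spring arm, enabling pawn control rotation, a lag distance cap and debug lag markers.
; Each mode function sets a target socket offset and clamped arm length, with camera lag disabled only for aim.
; Tick eases the spring arm toward those targets through interpolation, smoothing mode transitions.
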(event `self.ReceiveBeginPlay`
  (bind _asspring_arm_component (cast `SpringArmComponent` (`|GetArrayItem` (`self.GetParentComponents`))))
  (set `self.SpringArm` _asspring_arm_component)
  (set `SpringArmComponent.bUsePawnControlRotation` true (`self.SpringArm`))
  (set `SpringArmComponent.CameraLagMaxDistance` 50.0 (`self.SpringArm`))
  ;[1 1 1] Debug
  (set `SpringArmComponent.bDrawDebugLagMarkers` true (`self.SpringArm`)))

(event `self.ReceiveTick`
  (params (DeltaSeconds :type "Float (single-precision)"))
  (`self.UpdateCamera`))

(fn `GetTargetArmLength`
  (returns (ReturnValue :type "Float (double-precision)"))
  (return (`self.TargetArmLength`)))

(fn `SetTargetArmLength`
  (params (TargetArmLength :type "Float (double-precision)"))
  (returns (ReturnValue :type "Float (double-precision)"))
  (set `self.TargetArmLength` (`KismetMathLibrary.FClamp` (`local.TargetArmLength`) 0.0 900.0))
  (return (`self.TargetArmLength`)))

(fn `ToAimMode`
  (set `self.TargetSocketOffset` (`self.AIM_SOCKET_OFFSET`))
  (`self.SetTargetArmLength` (`self.AIM_ARM_LENGTH`))
  (set `SpringArmComponent.bEnableCameraLag` false (`self.SpringArm`)))

(fn `ToDefaultMode`
  (set `self.TargetSocketOffset` (`self.DEFAULT_SOCKET_OFFSET`))
  (`self.SetTargetArmLength` (`self.DEFAULT_ARM_LENGTH`))
  (set `SpringArmComponent.bEnableCameraLag` true (`self.SpringArm`)))

(fn `ToMeleeMode`
  (set `self.TargetSocketOffset` (`self.MELEE_SOCKET_OFFSET`))
  (`self.SetTargetArmLength` (`self.MELEE_ARM_LENGTH`))
  (set `SpringArmComponent.bEnableCameraLag` true (`self.SpringArm`)))

(fn `ToRangeMode`
  (set `self.TargetSocketOffset` (`self.RANGE_SOCKET_OFFSET`))
  (`self.SetTargetArmLength` (`self.RANGE_ARM_LENGTH`))
  (set `SpringArmComponent.bEnableCameraLag` true (`self.SpringArm`)))

(fn `UpdateCamera`
  (set `SpringArmComponent.TargetArmLength` (`KismetMathLibrary.FInterpTo` (`SpringArmComponent.TargetArmLength` (`self.SpringArm`)) (`self.TargetArmLength`) (`GameplayStatics.GetWorldDeltaSeconds`) 2.0) (`self.SpringArm`))
  (set `SpringArmComponent.SocketOffset` (`KismetMathLibrary.VInterpTo` (`SpringArmComponent.SocketOffset` (`self.SpringArm`)) (`self.TargetSocketOffset`) (`GameplayStatics.GetWorldDeltaSeconds`) 2.0) (`self.SpringArm`)))