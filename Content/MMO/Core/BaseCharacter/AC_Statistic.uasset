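; Character stat component that holds health, stamina and magic, flags death at zero health, and decides the Walk, Run or Sprint movement state.
; Sprint and walk inputs plus AC_Attack's combat-type and battle-state events drive the movement state machine, with sprint also gated by stamina.
; Movement changes set a signed stamina rate applied on Tick, delaying regeneration after a drain and broadcasting OnStaminaZero when depleted.
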(event `self.ReceiveBeginPlay`
  (bind _returnvalue (`Actor.GetComponentByClass` (`self.GetOwner`) "/Game/MMO/Core/BaseCharacter/AC_Attack.AC_Attack_C"))
  (add `self.OnMovementStateChanged` (`|CreateDelegate` :!event `OnMovementStateChanged_Event`))
  (`/Engine/EditorBlueprintResources/StandardMacros.IsValid` _returnvalue
    (:`Is Valid`
      (bind _output_get (set `self.OwnerAttackComp` _returnvalue))
      (add `/Game/MMO/Core/BaseCharacter/AC_Attack.OnCombatTypeChanged` _output_get (`|CreateDelegate` :!event `OnCombatTypeChanged_Event`))
      (add `/Game/MMO/Core/BaseCharacter/AC_Attack.OnBattleStateChanged` (`self.OwnerAttackComp`) (`|CreateDelegate` :!event `OnBattleStateChanged_Event`)))))

(event `self.ReceiveTick`
  (params (DeltaSeconds :type "Float (single-precision)"))
  (if (`self.RegenEnabled`)
    (`self.StaminaRegen`)))

(event `SprintBtnChangedEvent`
  (params (SprintBtn :type Boolean))
  (set `self.bSprintPressed` SprintBtn)
  (`self.UpdateMovementState`))

(event `WalkBtnChangedEvent`
  (params (WalkBtn :type Boolean))
  (set `self.bWalkPressed` WalkBtn)
  (`self.UpdateMovementState`))

(event `OnMovementStateChanged_Event` :!signature `self.OnMovementStateChanged`
  (params (MovementState :type "/Game/MMO/Core/BaseCharacter/E_MovementState Enum" :default "NewEnumerator1"))
  (bind _stamina_run_regen (`self.STAMINA_RUN_REGEN`))
  (if (< (`self.StaminaRegenVal`) 0.0)
    (set `self.StaminaRegenVal` 0.0)
    (`KismetSystemLibrary.Delay` (`self.StaminaRegenDelay`)))
  (set `self.StaminaRegenVal` (select `/Game/MMO/Core/BaseCharacter/E_MovementState` MovementState :`NewEnumerator1` _stamina_run_regen :`NewEnumerator2` _stamina_run_regen :`NewEnumerator3` (`self.STAMINA_SPRINT_REGEN`))))

(event `OnCombatTypeChanged_Event`
  (params (CombatType :type "/Game/MMO/Core/BaseCharacter/E_CombatType Enum" :default "NewEnumerator3") (OldCombatType :type "/Game/MMO/Core/BaseCharacter/E_CombatType Enum" :default "NewEnumerator3"))
  (set `self.CombatType` CombatType)
  (`self.UpdateMovementState`))

(event `OnBattleStateChanged_Event`
  (params (BattleState :type "/Game/MMO/Core/BaseCharacter/E_BattleState Enum" :default "NewEnumerator0"))
  (set `self.BattleState` BattleState)
  (`self.UpdateMovementState`))

(fn `GetCurrentHealth`
  (returns (ReturnValue :type "Float (double-precision)"))
  (return (`self.CurrentHealth`)))

(fn `GetCurrentMagic`
  (returns (ReturnValue :type "Float (double-precision)"))
  (return (`self.CurrentMagic`)))

(fn `GetCurrentStamina`
  (returns (ReturnValue :type "Float (double-precision)"))
  (return (`self.CurrentStamina`)))

(fn `GetDead`
  (returns (ReturnValue :type Boolean))
  (return (`self.bDead`)))

(fn `GetMaxHealth`
  (returns (ReturnValue :type "Float (double-precision)"))
  (return (`self.MaxHealth`)))

(fn `GetMaxMagic`
  (returns (ReturnValue :type "Float (double-precision)"))
  (return (`self.MaxMagic`)))

(fn `GetMaxStamina`
  (returns (ReturnValue :type "Float (double-precision)"))
  (return (`self.MaxStamina`)))

(fn `SetCurrentHealth`
  (params (Value :type "Float (double-precision)"))
  (returns (Output_Get :type "Float (double-precision)"))
  (bind _output_get (set `self.CurrentHealth` Value))
  (if (== _output_get 0.0)
    (set `self.bDead` true))
  (return (`self.CurrentHealth`)))

(fn `SetMaxHealth`
  (params (Value :type "Float (double-precision)"))
  (returns (Output_Get :type "Float (double-precision)"))
  (bind _output_get (set `self.MaxHealth` Value))
  (return _output_get))

(fn `StaminaRegen`
  (bind _returnvalue (+ (`self.CurrentStamina`) (* (`self.StaminaRegenVal`) (`GameplayStatics.GetWorldDeltaSeconds`))))
  (`/Engine/EditorBlueprintResources/StandardMacros.CompareFloat` (+ (`self.CurrentStamina`) (* (`self.StaminaRegenVal`) (`GameplayStatics.GetWorldDeltaSeconds`))) (`self.MaxStamina`)
    (:`>`
      (set `self.CurrentStamina` (`self.MaxStamina`) :!label _label))
    (:`==`
      (goto _label))
    (:`<`
      (if (<= _returnvalue 0.0)
        (set `self.CurrentStamina` 0.0)
        (set `self.StaminaRegenVal` (`self.STAMINA_RUN_REGEN`))
        (`self.OnStaminaZero`)
        (else
          (set `self.CurrentStamina` _returnvalue))))))