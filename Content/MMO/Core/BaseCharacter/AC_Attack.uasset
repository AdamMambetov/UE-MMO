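; Actor component that manages a character's melee combo attacks, battle mode, blocking and switching between sword-and-shield and crossbow.
; Condition functions gate each action on animation, movement, death or battle state, and battle mode toggles controller-yaw versus movement-oriented rotation.
; Attacks run a two-hit combo state machine that buffers the next input for SaveCombo to replay.
; It talks to the owner and AnimInstance through message calls, polling animation state on Tick.
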(event `self.ReceiveBeginPlay`
  (bind _ascharacter (cast `Character` (`self.GetOwner`)))
  (set `self.Owner` _ascharacter)
  (set `self.AnimInstance` (`SkeletalMeshComponent.GetAnimInstance` (`Character.Mesh` (`self.Owner`)))))

(event `self.ReceiveTick`
  (params (DeltaSeconds :type "Float (single-precision)"))
  (bind _returnvalue (message `/Game/MMO/Core/BaseCharacter/BPI_AnimBaseCharacter.GetAnimPlaying` (`self.AnimInstance`)))
  (set `self.bAnimPlaying` _returnvalue))

(fn `Attack`
  (bind _returnvalue (message `/Game/MMO/Core/BaseCharacter/BPI_BaseCharacter.GetDirection` (`self.Owner`)))
  (`self.ComboAttack` _returnvalue))

(fn `BattleModeConditions`
  (returns (bReturnValue :type Boolean))
  (return (and (`|EnumEquality` (`self.BattleState`) "NewEnumerator0") (not (`self.bAnimPlaying`)) (`CharacterMovementComponent.IsWalking` (`Character.CharacterMovement` (`self.Owner`))))))

(fn `BlockConditions`
  (returns (bReturnValue :type Boolean))
  (locals (l_dead :type Boolean :default false))
  (bind _returnvalue (message `/Game/MMO/Core/BaseCharacter/BPI_BaseCharacter.GetDead` (`self.Owner`)))
  (set `local.l_dead` _returnvalue)
  (return (and (not (`self.bAnimPlaying`)) (`CharacterMovementComponent.IsWalking` (`Character.CharacterMovement` (`self.Owner`))) (`self.bBattleMode`) (not (`local.l_dead`)))))

(fn `ChangeCombatType`
  (params (CombatType :type "/Game/MMO/Core/BaseCharacter/E_CombatType Enum" :default "NewEnumerator2"))
  (set `self.CombatType` CombatType)
  (return))

(fn `ChangeWeapon`
  (if (`self.ChangeWeaponCondition`)
    (set `self.OldCombatType` (`self.CombatType`))
    (switch `/Game/MMO/Core/BaseCharacter/E_CombatType` (`self.CombatType`)
      (:`NewEnumerator0`
        (set `self.CombatType` "NewEnumerator1"))
      (:`NewEnumerator1`
        (set `self.CombatType` "NewEnumerator0")))
    (message `/Game/MMO/Core/BaseCharacter/BPI_AnimBaseCharacter.ChangeWeapon` (`self.AnimInstance`))))

(fn `ChangeWeaponCondition`
  (returns (ReturnValue :type Boolean))
  (return (not (`self.bAnimPlaying`))))

(fn `ComboAttack`
  (params (Direction :type "/Game/MMO/Core/BaseCharacter/E_DirectionState Enum" :default "NewEnumerator0"))
  (bind _breturnvalue (`self.ComboAttackConditions`))
  (if (and _breturnvalue (`self.bComboAttackPermission`))
    (set `self.bComboAttackPermission` false)
    (bind _result (`/Engine/EditorBlueprintResources/StandardMacros.IncrementInt` (`self.ComboCount`))
      (:`  `
        (switch `int` _result
          (:`Default`
            (message `/Game/MMO/Core/BaseCharacter/BPI_BaseCharacter.ResetCombo` (`self.Owner`)))
          (:`1`
            (message `/Game/MMO/Core/BaseCharacter/BPI_AnimBaseCharacter.AttackPlay` (`self.AnimInstance`) (`self.ComboCount`) (`self.bComboAttackHard`) (`local.Direction`)))
          (:`2`
            (message `/Game/MMO/Core/BaseCharacter/BPI_AnimBaseCharacter.AttackPlay` (`self.AnimInstance`) (`self.ComboCount`) (`self.bComboAttackHard`) (`local.Direction`))))))))

(fn `ComboAttackConditions`
  (returns (bReturnValue :type Boolean))
  (locals (lDead :type Boolean) (lAttackPlaying :type Boolean))
  (bind _returnvalue (message `/Game/MMO/Core/BaseCharacter/BPI_BaseCharacter.GetDead` (`self.Owner`)))
  (set `local.lDead` _returnvalue)
  (bind _returnvalue_2 (message `/Game/MMO/Core/BaseCharacter/BPI_AnimBaseCharacter.GetAttackPlaying` (`SkeletalMeshComponent.GetAnimInstance` (`Character.Mesh` (`self.Owner`)))))
  (set `local.lAttackPlaying` _returnvalue_2)
  (if (and (not (`local.lDead`)) (`|EnumEquality` (`self.CombatType`) "NewEnumerator0") (`|EnumInequality` (`self.BattleState`) "NewEnumerator1") (== (`self.bAnimPlaying`) (`local.lAttackPlaying`)))
    (if (`self.bBattleMode`)
      (switch `/Game/MMO/Core/BaseCharacter/E_ComboAttackState` (`self.ComboAttackState`)
        (:`NewEnumerator0`
          (set `self.bComboAttackPermission` true)
          (set `self.ComboAttackState` "NewEnumerator1")
          (return true))
        (:`NewEnumerator1`
          (set `self.ComboAttackState` "NewEnumerator2"))
        (:`NewEnumerator2`
          _))
      (if (not (`self.bAnimPlaying`))
        (message `/Game/MMO/Core/BaseCharacter/BPI_BaseCharacter.ResetCombo` (`self.Owner`))
        (return false)
        (else
          (return true)))
      (else
        (message `/Game/MMO/Core/BaseCharacter/BPI_BaseCharacter.EnableBattleMode` (`self.Owner`))
        (return false)))
    (else
      (return false))))

(fn `DisableBattleMode`
  (returns (bReturnValue :type Boolean))
  (if (`self.bBattleMode`)
    (if (`self.BattleModeConditions`)
      (set `self.bBattleMode` false)
      (set `Pawn.bUseControllerRotationYaw` false (`self.Owner`))
      (set `CharacterMovementComponent.bOrientRotationToMovement` true (`Character.CharacterMovement` (`self.Owner`)))
      (return true)
      (else
        (return false)))
    (else
      (return false))))

(fn `DisableBlock`
  (if (`|EnumEquality` "NewEnumerator1" (`self.BattleState`))
    (if (`self.BlockConditions`)
      (set `self.BattleState` "NewEnumerator0")
      (return)
      (else
        (return)))
    (else
      (return))))

(fn `EnableBattleMode`
  (returns (bReturnValue :type Boolean))
  (if (not (`self.bBattleMode`))
    (if (`self.BattleModeConditions`)
      (set `self.bBattleMode` true)
      (set `Pawn.bUseControllerRotationYaw` true (`self.Owner`))
      (set `CharacterMovementComponent.bOrientRotationToMovement` false (`Character.CharacterMovement` (`self.Owner`)))
      (return true)
      (else
        (return false)))
    (else
      (return false))))

(fn `EnableBlock`
  (if (`|EnumEquality` "NewEnumerator0" (`self.BattleState`))
    (if (`self.BlockConditions`)
      (set `self.BattleState` "NewEnumerator1")
      (return)
      (else
        (return)))
    (else
      (return))))

(fn `ResetCombo`
  (set `self.ComboCount` 0)
  (set `self.ComboAttackState` "NewEnumerator0")
  (set `self.bComboAttackPermission` false))

(fn `SaveCombo`
  (if (`self.SaveComboConditions`)
    (set `self.ComboAttackState` "NewEnumerator1")
    (set `self.bComboAttackPermission` true)
    (`self.ComboAttack` "NewEnumerator0")))

(fn `SaveComboConditions`
  (returns (bReturnValue :type Boolean))
  (return (`|EnumEquality` "NewEnumerator2" (`self.ComboAttackState`))))