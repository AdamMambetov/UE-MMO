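; Actor component that tracks the weapon and armor actors currently worn by its owning character and exposes a getter for each slot.
; UpdateWeapon and UpdateArmor destroy the slot's actor when Equipped is true; otherwise they spawn and attach a new one.
; Spawning is delegated to freshly spawned use-case actors owned by the character, with results stored by weapon type or armor chunk.
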(event `self.ReceiveBeginPlay`
  (bind _ascharacter (cast `Character` (`self.GetOwner`)))
  (set `self.Owner` _ascharacter))

(fn `GetCurrentChest`
  (returns (ReturnValue :type "/Game/MMO/Core/Inventory/BP_Base_Armor Object Reference"))
  (return (`self.CurrentChest`)))

(fn `GetCurrentGloves`
  (returns (ReturnValue :type "/Game/MMO/Core/Inventory/BP_Base_Armor Object Reference"))
  (return (`self.CurrentGloves`)))

(fn `GetCurrentHelmet`
  (returns (ReturnValue :type "/Game/MMO/Core/Inventory/BP_Base_Armor Object Reference"))
  (return (`self.CurrentHelmet`)))

(fn `GetCurrentMeleeWeapon`
  (returns (ReturnValue :type "/Game/MMO/Core/Inventory/BP_BaseMeleeWeapon Object Reference"))
  (return (`self.CurrentMeleeWeapon`)))

(fn `GetCurrentRangeWeapon`
  (returns (ReturnValue :type "/Game/MMO/Core/Inventory/BP_BaseRangeWeapon Object Reference"))
  (return (`self.CurrentRangeWeapon`)))

(fn `GetCurrentShield`
  (returns (ReturnValue :type "/Game/MMO/Core/Inventory/BP_Base_Armor Object Reference"))
  (return (`self.CurrentShield`)))

(fn `GetCurrentShoes`
  (returns (ReturnValue :type "/Game/MMO/Core/Inventory/BP_Base_Armor Object Reference"))
  (return (`self.CurrentShoes`)))

(fn `GetCurrentShoulders`
  (returns (ReturnValue :type "/Game/MMO/Core/Inventory/BP_Base_Armor Object Reference"))
  (return (`self.CurrentShoulders`)))

(fn `UpdateArmor`
  (params (ArmorInfo :type "/Game/MMO/Core/Inventory/S_Armor_Info Structure") (bEquipped :type Boolean))
  (if bEquipped
    (`Actor.K2_DestroyActor` (select `/Game/MMO/Core/Inventory/E_ArmorType` (`.Chunk_2_58004BF94078A5E646A77FA0CD68DCFB` (break `/Game/MMO/Core/Inventory/S_Armor_Info` (`local.ArmorInfo`))) :`NewEnumerator0` (`self.CurrentHelmet`) :`NewEnumerator1` (`self.CurrentChest`) :`NewEnumerator2` (`self.CurrentGloves`) :`NewEnumerator4` (`self.CurrentShoes`) :`NewEnumerator5` (`self.CurrentShoulders`) :`NewEnumerator6` (`self.CurrentShield`) :!type "Actor Object Reference"))
    (else
      (bind _returnvalue (`|SpawnActorFromClass` "/Game/MMO/Core/UseCases/ArmorSpawnUseCase.ArmorSpawnUseCase_C" (`KismetMathLibrary.MakeTransform` (0.0 0.0 0.0)) "Undefined" "OverrideRootScale" (`self.Owner`) null))
      (bind _returnvalue_2 (`/Game/MMO/Core/UseCases/ArmorSpawnUseCase.SpawnArmorAndAttach` _returnvalue (`.Class_12_530F362D45E80F8D63F492B6669640E1` (break `/Game/MMO/Core/Inventory/S_Armor_Info` (`local.ArmorInfo`)))))
      (switch `/Game/MMO/Core/Inventory/E_ArmorType` (`.Chunk_2_58004BF94078A5E646A77FA0CD68DCFB` (break `/Game/MMO/Core/Inventory/S_Armor_Info` (`local.ArmorInfo`)))
        (:`NewEnumerator0`
          (set `self.CurrentHelmet` _returnvalue_2))
        (:`NewEnumerator1`
          (set `self.CurrentChest` _returnvalue_2))
        (:`NewEnumerator2`
          (set `self.CurrentGloves` _returnvalue_2))
        (:`NewEnumerator4`
          (set `self.CurrentShoes` _returnvalue_2))
        (:`NewEnumerator5`
          (set `self.CurrentShoulders` _returnvalue_2))
        (:`NewEnumerator6`
          (set `self.CurrentShield` _returnvalue_2))))))

(fn `UpdateWeapon`
  (params (WeaponInfo :type "/Game/MMO/Core/Inventory/S_Weapon_Info Structure") (bEquipped :type Boolean))
  (if bEquipped
    (`Actor.K2_DestroyActor` (select `/Game/MMO/Core/Inventory/E_WeaponType` (`.WeaponType_13_58004BF94078A5E646A77FA0CD68DCFB` (break `/Game/MMO/Core/Inventory/S_Weapon_Info` (`local.WeaponInfo`))) :`NewEnumerator0` (`self.CurrentMeleeWeapon`) :`NewEnumerator1` (`self.CurrentRangeWeapon`) :!type "Actor Object Reference"))
    (else
      (bind _returnvalue (`|SpawnActorFromClass` "/Game/MMO/Core/UseCases/WeaponSpawnUseCase.WeaponSpawnUseCase_C" (`KismetMathLibrary.MakeTransform` (0.0 0.0 0.0)) "Undefined" "OverrideRootScale" (`self.Owner`) null))
      (switch `/Game/MMO/Core/Inventory/E_WeaponType` (`.WeaponType_13_58004BF94078A5E646A77FA0CD68DCFB` (break `/Game/MMO/Core/Inventory/S_Weapon_Info` (`local.WeaponInfo`)))
        (:`NewEnumerator0`
          (bind _returnvalue_2 (`/Game/MMO/Core/UseCases/WeaponSpawnUseCase.SpawnMeleeWeaponAndAttach` _returnvalue (`.Class_19_DA7F0F494B3B5E77D91B0E9A95BC8065` (break `/Game/MMO/Core/Inventory/S_Weapon_Info` (`local.WeaponInfo`)))))
          (set `self.CurrentMeleeWeapon` _returnvalue_2))
        (:`NewEnumerator1`
          (bind _returnvalue_3 (`/Game/MMO/Core/UseCases/WeaponSpawnUseCase.SpawnRangeWeaponAndAttach` _returnvalue (`.Class_19_DA7F0F494B3B5E77D91B0E9A95BC8065` (break `/Game/MMO/Core/Inventory/S_Weapon_Info` (`local.WeaponInfo`)))))
          (set `self.CurrentRangeWeapon` _returnvalue_3))))))