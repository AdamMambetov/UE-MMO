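; Actor component in BaseCharacter that tracks whether the Attack, Hard Attack and Aim, and Block buttons are held.
; PressKey routes a key and pressed flag into the InputAction macro, which sets the matching boolean and calls its per-button change dispatcher.
; The IsNotEqual macro filters out None and unchanged states, so dispatchers fire only on real transitions.
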(fn `PressKey`
  (params (Pressed :type Boolean) (Key :type "/Game/MMO/Core/BaseCharacter/E_ActionKeys Enum" :default "NewEnumerator1"))
  (if Pressed
    (`self.InputAction` Key :!label _label)
    (else
      (goto _label :!via `Released`))))