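; Base melee weapon actor that deals damage through separate attack and block collision components.
; Attack/AttackEnd and Block/BlockEnd toggle query-only collision on each component.
; Attack overlaps apply WeaponInfo damage to damageable non-owners, then close the hit window; block overlaps deal token damage without an owner check.
; Tick prints the damage collision state and owner name for debugging.
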(event `self.ReceiveTick`
  (params (DeltaSeconds :type "Float (single-precision)"))
  (`KismetSystemLibrary.PrintString` (`KismetStringLibrary.Concat_StrStr` (`KismetStringLibrary.Conv_BoolToString` (`PrimitiveComponent.K2_IsCollisionEnabled` (`self.DamageCollision`))) (`KismetSystemLibrary.GetDisplayName` (`self.GetOwner`))) true true (struct :`G` 0.66 :`B` 1.0 :`A` 1.0) 0.0))

(event `self.DamageCollision.OnComponentBeginOverlap`
  (params (OverlappedComponent :type "PrimitiveComponent Object Reference") (OtherActor :type "Actor Object Reference") (OtherComp :type "PrimitiveComponent Object Reference") (OtherBodyIndex :type Integer) (bFromSweep :type Boolean) (SweepResult :type "HitResult Structure (by ref)"))
  (if (and (`Actor.bCanBeDamaged` OtherActor) (!= OtherActor (`self.GetOwner`)))
    (`GameplayStatics.ApplyDamage` OtherActor (`.Damage_15_FE9AE930450442E12D87738F7FACF334` (break `/Game/MMO/Core/Inventory/S_Weapon_Info` (`self.WeaponInfo`))) null self)
    (`self.AttackEnd`)))

(event `self.BlockCollision.OnComponentBeginOverlap`
  (params (OverlappedComponent :type "PrimitiveComponent Object Reference") (OtherActor :type "Actor Object Reference") (OtherComp :type "PrimitiveComponent Object Reference") (OtherBodyIndex :type Integer) (bFromSweep :type Boolean) (SweepResult :type "HitResult Structure (by ref)"))
  (if (`Actor.bCanBeDamaged` OtherActor)
    (`GameplayStatics.ApplyDamage` OtherActor 1.0 null self)))

(fn `Attack`
  (`PrimitiveComponent.SetCollisionEnabled` (`self.DamageCollision`) "QueryOnly"))

(fn `AttackEnd`
  (`PrimitiveComponent.SetCollisionEnabled` (`self.DamageCollision`) "NoCollision"))

(fn `Block`
  (`PrimitiveComponent.SetCollisionEnabled` (`self.BlockCollision`) "QueryOnly"))

(fn `BlockEnd`
  (`PrimitiveComponent.SetCollisionEnabled` (`self.BlockCollision`) "NoCollision"))

(fn `UserConstructionScript`
  (`parent.UserConstructionScript`))