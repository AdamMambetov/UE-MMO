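; Base weapon actor for the inventory system, supporting both melee-style collision attacks and bolt shots.
; Construction loads its data from DT_WeaponList by InitialID, sets amount and mesh, and disables DamageCollision until Attack enables it.
; Shot traces from the owner's camera for BPI_MainCharacter owners, otherwise from BoltSocket toward the supplied End.
; It then spawns BP_Bolt at the socket aimed at the trace result, leaving persistent debug lines.
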(fn `Attack`
  (`PrimitiveComponent.SetCollisionEnabled` (`self.DamageCollision`) "QueryOnly"))

(fn `GetItemInfo`
  (returns (Type :type "/Game/MMO/Core/Inventory/E_ItemType Enum") (ID :type Name) (Amount :type Integer))
  (bind ((`Type_11_A385B47849A45CE53C8EF9BFBE7210D4` _type) (`Amount_49_D1E29AF04498C178B74986AAD5610193` _amount) (`ID_50_BA06E0BD4E97D16461377CB9BF36CE2D` _id)) (break `/Game/MMO/Core/Inventory/S_Item_Info` (`.ItemInfo_9_747206B9457C40D5BDF581B82BDB6F08` (break `/Game/MMO/Core/Inventory/S_Weapon_Info` (`self.WeaponInfo`)))))
  (return _type _id _amount))

(fn `Shot`
  (params (End :type "Vector Structure"))
  (locals (L_Start :type "Vector Structure") (L_End :type "Vector Structure"))
  (bind _returnvalue (`SceneComponent.GetSocketLocation` (`self.SkeletalMesh`) "BoltSocket"))
  (bind _returnvalue_2 (`self.GetComponentByClass` (`self.GetOwner`) "/Script/Engine.CameraComponent"))
  (`|ExecutionSequence`
    (:`then_0`
      (if (`KismetSystemLibrary.DoesImplementInterface` (`self.GetOwner`) "/Game/MMO/Characters/MainCharacter/BPI_MainCharacter.BPI_MainCharacter_C")
        (set `local.L_Start` (`SceneComponent.K2_GetComponentLocation` _returnvalue_2))
        (set `local.L_End` (+ (`local.L_Start`) (* (`SceneComponent.GetForwardVector` _returnvalue_2) 100000.0)))
        (else
          (set `local.L_Start` (`SceneComponent.GetSocketLocation` (`self.SkeletalMesh`) "BoltSocket"))
          (set `local.L_End` (`local.End`)))))
    (:`then_1`
      (bind (_outhit _returnvalue_3) (`KismetSystemLibrary.LineTraceSingleForObjects` :`Start` (`local.L_Start`) :`End` (`local.L_End`) :`ObjectTypes` (`|MakeArray` "ObjectTypeQuery1" "ObjectTypeQuery2" "ObjectTypeQuery3" "ObjectTypeQuery4" "ObjectTypeQuery7" :!type "EObjectTypeQuery Enum") :`DrawDebugType` "Persistent"))
      (bind (_bblockinghit _binitialoverlap _time _distance _location _impactpoint _normal _impactnormal _physmat _hitactor _hitcomponent _hitbonename _hititem _elementindex _faceindex _tracestart _traceend) (`GameplayStatics.BreakHitResult` _outhit))
      (`|SpawnActorFromClass` "/Game/MMO/Core/BaseCharacter/BP_Bolt.BP_Bolt_C" (`KismetMathLibrary.MakeTransform` _returnvalue (`KismetMathLibrary.FindLookAtRotation` _returnvalue (`KismetMathLibrary.SelectVector` _location _traceend _returnvalue_3))) "Undefined" "OverrideRootScale" (`self.GetOwner`) null))))

(fn `UserConstructionScript`
  (`parent.UserConstructionScript`)
  (bind _returnvalue (`|GetDataTableRow` "/Game/MMO/Core/Inventory/DT_WeaponList.DT_WeaponList" (`self.InitialID`))
    (:`then`
      (bind _output_get (set `self.WeaponInfo` _returnvalue))
      (setmembers `/Game/MMO/Core/Inventory/S_Item_Info` :`StructRef` (`.ItemInfo_9_747206B9457C40D5BDF581B82BDB6F08` (break `/Game/MMO/Core/Inventory/S_Weapon_Info` _output_get)) :`Amount` (`self.InitialAmount`))
      (`SkinnedMeshComponent.SetSkinnedAssetAndUpdate` (`self.SkeletalMesh`) (`.SkeletalMesh_51_44579ECC489E180B8BC740AADCECDAAF` (break `/Game/MMO/Core/Inventory/S_Item_Info` (`.ItemInfo_9_747206B9457C40D5BDF581B82BDB6F08` (break `/Game/MMO/Core/Inventory/S_Weapon_Info` (`self.WeaponInfo`))))) true)
      (`PrimitiveComponent.SetCollisionEnabled` (`self.DamageCollision`) "NoCollision"))))