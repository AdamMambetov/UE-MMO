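; Base Blueprint for potion items in the MMO inventory system, configured from a data table.
; The construction script looks up InitialID in DT_PotionList, overrides the amount with InitialAmount, and stores item info and effects in PotionInfo.
; It then applies the row's skeletal mesh, so the potion's appearance follows its data.
; GetItemInfo exposes the stored type, ID and amount.
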(fn `GetItemInfo`
  (returns (Type :type "/Game/MMO/Core/Inventory/E_ItemType Enum") (ID :type Name) (Amount :type Integer))
  (bind ((`Type_11_A385B47849A45CE53C8EF9BFBE7210D4` _type) (`Amount_49_D1E29AF04498C178B74986AAD5610193` _amount) (`ID_50_BA06E0BD4E97D16461377CB9BF36CE2D` _id)) (break `/Game/MMO/Core/Inventory/S_Item_Info` (`.ItemInfo_14_7E8F48144F0F01654500E084A85436C5` (break `/Game/MMO/Core/Inventory/S_Potion_Info` (`self.PotionInfo`)))))
  (return _type _id _amount))

(fn `UserConstructionScript`
  (`parent.UserConstructionScript`)
  (bind _returnvalue (`|GetDataTableRow` "/Game/MMO/Core/Inventory/DT_PotionList.DT_PotionList" (`self.InitialID`))
    (:`then`
      (bind (_iteminfo _effects) (break `/Game/MMO/Core/Inventory/S_Potion_Info` _returnvalue))
      (bind _structout (setmembers `/Game/MMO/Core/Inventory/S_Item_Info` :`StructRef` _iteminfo :`Amount` (`self.InitialAmount`)))
      (bind _output_get (set `self.PotionInfo` (make `/Game/MMO/Core/Inventory/S_Potion_Info` _structout _effects)))
      (`SkinnedMeshComponent.SetSkinnedAssetAndUpdate` (`self.SkeletalMesh`) (`.SkeletalMesh_51_44579ECC489E180B8BC740AADCECDAAF` (break `/Game/MMO/Core/Inventory/S_Item_Info` (`.ItemInfo_14_7E8F48144F0F01654500E084A85436C5` (break `/Game/MMO/Core/Inventory/S_Potion_Info` _output_get)))) true))))