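; Inventory component that holds items and amounts in a slot array, sized to AmountOfSlots on BeginPlay.
; AddItem puts stackable items into the first partial matching stack or else an empty slot, and non-stackable items one per slot.
; It calls itself recursively for amounts beyond one slot, returning success and any unplaced Rest.
; Helper functions find free stacks and empty slots and report item info or amount by index.
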(event `self.ReceiveBeginPlay`
  (`KismetArrayLibrary.Array_Resize` (`self.Inventory`) (`self.AmountOfSlots`)))

(fn `AddItem`
  (params (Item :type "/Game/MMO/Core/Inventory/BP_MasterItem Object Reference") (Amount :type Integer))
  (returns (ReturnValue :type Boolean) (Rest :type Integer))
  (locals (local_FoundIndex :type Integer :default 0))
  (bind (_returnvalue _index) (`self.SearchEmptySlot`))
  (bind (_returnvalue_2 _index_2) (`self.SearchEmptySlot`))
  (bind _returnvalue_3 (+ (`.Amount_5_25F50AA64A4F2824DD1C49AAA508C9E6` (break `/Game/MMO/Core/Inventory/S_InventorySlot` (`|GetArrayItem` (`self.Inventory`) (`local.local_FoundIndex`)))) (`local.Amount`)))
  (if (`.Stacked_27_B9C41EB0416DBFA24E1E75A6CD16E5AA` (break `/Game/MMO/Core/Inventory/S_ItemInfo` (`/Game/MMO/Core/Inventory/BP_MasterItem.ItemInfo` Item)))
    ;[1 1 1] Item Stacked
    (bind (_returnvalue_4 _index_3) (`self.SearchFreeStack` (`local.Item`)))
    (if _returnvalue_4
      (set `local.local_FoundIndex` _index_3)
      (if (> _returnvalue_3 (`self.MaxStackSize`))
        (`KismetArrayLibrary.Array_Set` (`self.Inventory`) (`local.local_FoundIndex`) (make `/Game/MMO/Core/Inventory/S_InventorySlot` (`local.Item`) (`self.MaxStackSize`)))
        (bind (_returnvalue_5 _rest) (`self.AddItem` (`local.Item`) (- _returnvalue_3 (`self.MaxStackSize`))))
        (return true _rest)
        (else
          (`KismetArrayLibrary.Array_Set` (`self.Inventory`) (`local.local_FoundIndex`) (make `/Game/MMO/Core/Inventory/S_InventorySlot` (`local.Item`) _returnvalue_3))
          (return true 0)))
      (elif _returnvalue_2
        (set `local.local_FoundIndex` _index_2)
        (if (> (`local.Amount`) (`self.MaxStackSize`))
          (`KismetArrayLibrary.Array_Set` (`self.Inventory`) (`local.local_FoundIndex`) (make `/Game/MMO/Core/Inventory/S_InventorySlot` (`local.Item`) (`self.MaxStackSize`)))
          (bind (_returnvalue_6 _rest_2) (`self.AddItem` (`local.Item`) (- (`local.Amount`) (`self.MaxStackSize`))))
          (return true _rest_2)
          (else
            (`KismetArrayLibrary.Array_Set` (`self.Inventory`) (`local.local_FoundIndex`) (make `/Game/MMO/Core/Inventory/S_InventorySlot` (`local.Item`) (`local.Amount`)))
            (return true 0)))
        (else
          (return false (`local.Amount`)))))
    (else
      ;[1 1 1] If Item Not Stacked
      (if _returnvalue
        (bind _output_get (set `local.local_FoundIndex` _index))
        (`KismetArrayLibrary.Array_Set` (`self.Inventory`) _output_get (make `/Game/MMO/Core/Inventory/S_InventorySlot` (`local.Item`) 1))
        (if (> (`local.Amount`) 1)
          (bind (_returnvalue_7 _rest_3) (`self.AddItem` (`local.Item`) (- (`local.Amount`) 1)))
          (return true _rest_3)
          (else
            (return true 0)))
        (else
          (return false (`local.Amount`)))))))

(fn `GetAmountAtIndex`
  (params (Index :type Integer))
  (returns (Amount :type Integer))
  (return (`.Amount_5_25F50AA64A4F2824DD1C49AAA508C9E6` (break `/Game/MMO/Core/Inventory/S_InventorySlot` (`|GetArrayItem` (`self.Inventory`) (`local.Index`))))))

(fn `GetItemInfoAtIndex`
  (params (Index :type Integer))
  (returns (ReturnValue :type Boolean) (ItemInfo :type "/Game/MMO/Core/Inventory/S_ItemInfo Structure") (Amount :type Integer))
  (bind (_item _amount) (break `/Game/MMO/Core/Inventory/S_InventorySlot` (`|GetArrayItem` (`self.Inventory`) (`local.Index`))))
  (`/Engine/EditorBlueprintResources/StandardMacros.IsValid` _item
    (:`Is Valid`
      (return true (`/Game/MMO/Core/Inventory/BP_MasterItem.ItemInfo` _item) _amount))
    (:`Is Not Valid`
      (return false (struct) 0))))

(fn `IsSlotEmpty`
  (params (Index :type Integer))
  (returns (ReturnValue :type Boolean))
  (return (not (`KismetSystemLibrary.IsValid` (`.Item_7_F10F327A45771CDE63C8CE9CAA764CF7` (break `/Game/MMO/Core/Inventory/S_InventorySlot` (`|GetArrayItem` (`self.Inventory`) Index)))))))

(fn `SearchEmptySlot`
  (returns (ReturnValue :type Boolean) (Index :type Integer))
  (locals (local_bool :type Boolean) (localIndex :type Integer))
  (for (_array_element _array_index) (`self.Inventory`)
    (if (not (`KismetSystemLibrary.IsValid` (`.Item_7_F10F327A45771CDE63C8CE9CAA764CF7` (break `/Game/MMO/Core/Inventory/S_InventorySlot` _array_element))))
      (set `local.local_bool` true)
      (set `local.localIndex` _array_index)
      (break)))
  (return (`local.local_bool`) (`local.localIndex`)))

(fn `SearchFreeStack`
  (params (Item :type "/Game/MMO/Core/Inventory/BP_MasterItem Object Reference"))
  (returns (ReturnValue :type Boolean) (Index :type Integer))
  (locals (local_bool :type Boolean) (local_index :type Integer))
  (for (_array_element _array_index) (`self.Inventory`)
    (bind (_item _amount) (break `/Game/MMO/Core/Inventory/S_InventorySlot` _array_element))
    (if (and (`KismetSystemLibrary.IsValid` _item) (== _item (`local.Item`)) (< _amount (`self.MaxStackSize`)))
      (set `local.local_bool` true)
      (set `local.local_index` _array_index)
      (break)))
  (return (`local.local_bool`) (`local.local_index`)))