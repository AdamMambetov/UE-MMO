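; Base ranged weapon for the inventory system that fires a BP_Bolt projectile from the mesh's BoltSocket.
; Shot line-traces from the camera for owners implementing BPI_MainCharacter, or from the socket toward a supplied end point for others.
; The bolt aims at the hit point if it lies beyond MINDISTANCE, otherwise at the trace end.
; Persistent trace drawing and a distance printout remain as debug output.
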(fn `Shot`
  (params (End :type "Vector Structure"))
  (locals (L_Start :type "Vector Structure") (L_End :type "Vector Structure"))
  (bind _returnvalue (`SceneComponent.GetSocketLocation` (`self.SkeletalMesh`) "BoltSocket"))
  (bind _returnvalue_2 (`self.GetComponentByClass` (`self.GetOwner`) "/Script/Engine.CameraComponent"))
  (`|ExecutionSequence`
    (:`then_0`
      (if (`KismetSystemLibrary.DoesImplementInterface` (`self.GetOwner`) "/Game/MMO/Characters/MainCharacter/BPI_MainCharacter.BPI_MainCharacter_C")
        (set `local.L_Start` (`SceneComponent.K2_GetComponentLocation` _returnvalue_2))
        (set `local.L_End` (+ (`local.L_Start`) (* (`SceneComponent.GetForwardVector` _returnvalue_2) 100000.0)))
        (else
          (set `local.L_Start` (`SceneComponent.GetSocketLocation` (`self.SkeletalMesh`) "BoltSocket"))
          (set `local.L_End` (`local.End`)))))
    (:`then_1`
      (bind (_outhit _returnvalue_3) (`KismetSystemLibrary.LineTraceSingleForObjects` (`local.L_Start`) (`local.L_End`) (`|MakeArray` "ObjectTypeQuery1" "ObjectTypeQuery2" "ObjectTypeQuery3" "ObjectTypeQuery4" "ObjectTypeQuery7" :!type "EObjectTypeQuery Enum") false (`|MakeArray` (`self.GetOwner`)) "Persistent"))
      (bind (_bblockinghit _binitialoverlap _time _distance _location _impactpoint _normal _impactnormal _physmat _hitactor _hitcomponent _hitbonename _hititem _elementindex _faceindex _tracestart _traceend) (`GameplayStatics.BreakHitResult` _outhit))
      (bind _returnvalue_4 (and (> _distance (`self.MIN_DISTANCE`)) _returnvalue_3))
      (`KismetSystemLibrary.PrintString` (`KismetStringLibrary.Concat_StrStr` (`KismetStringLibrary.Conv_DoubleToString` _distance) " > " (`KismetStringLibrary.Conv_DoubleToString` (`self.MIN_DISTANCE`)) (`KismetStringLibrary.Conv_BoolToString` _returnvalue_4)))
      (`|SpawnActorFromClass` "/Game/MMO/Core/Inventory/Weapon/BP_Bolt.BP_Bolt_C" (`KismetMathLibrary.MakeTransform` _returnvalue (`KismetMathLibrary.FindLookAtRotation` _returnvalue (`KismetMathLibrary.SelectVector` _location _traceend _returnvalue_4))) "Undefined" "OverrideRootScale" (`self.GetOwner`) null))))

(fn `UserConstructionScript`
  (`parent.UserConstructionScript`))