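; BP_Weapon_Sword is a melee sword weapon that deals damage to characters its collision touches.
; When DamageCollision begins overlapping an actor other than the owner that implements BPI_BaseCharacter, it applies the damage value from WeaponInfo.
; It then disables that collision, so further overlaps deal no damage until collision is re-enabled outside this graph.
; The construction script only calls the parent's.
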(event `self.DamageCollision.OnComponentBeginOverlap`
  (params (OverlappedComponent :type "PrimitiveComponent Object Reference") (OtherActor :type "Actor Object Reference") (OtherComp :type "PrimitiveComponent Object Reference") (OtherBodyIndex :type Integer) (bFromSweep :type Boolean) (SweepResult :type "HitResult Structure (by ref)"))
  (if (and (`KismetSystemLibrary.DoesImplementInterface` OtherActor "/Game/MMO/Core/BaseCharacter/BPI_BaseCharacter.BPI_BaseCharacter_C") (!= OtherActor (`self.GetOwner`)))
    (`GameplayStatics.ApplyDamage` null (`.Damage_15_FE9AE930450442E12D87738F7FACF334` (break `/Game/MMO/Core/Inventory/S_Weapon_Info` (`self.WeaponInfo`))))
    (`PrimitiveComponent.SetCollisionEnabled` (`self.DamageCollision`) "NoCollision")))

(fn `UserConstructionScript`
  (`parent.UserConstructionScript`))