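; Base pickup actor for inventory items that an interactor can collect.
; The construction script looks up InitialID in the armor, potion and weapon data tables in turn, storing the first match as ItemInfo and applying its static mesh.
; On Interaction, it passes the item's type, ID and amount to the interactor's AddItem, destroying itself only when the add succeeds with nothing left over.
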(event `/Game/MMO/Core/Inventory/BPI_Interact.Interaction`
  (params (Interactor :type "/Game/MMO/Core/BaseCharacter/BPI_BaseCharacter Interface"))
  (bind (_type _id _amount) (`self.GetItemInfo`))
  (bind (_breturnvalue _rest) (`/Game/MMO/Core/BaseCharacter/BPI_BaseCharacter.AddItem` Interactor _type _id _amount))
  (if (and _breturnvalue (== _rest 0))
    (`self.K2_DestroyActor`)))

(fn `GetItemInfo`
  (returns (Type :type "/Game/MMO/Core/Inventory/E_ItemType Enum") (ID :type Name) (Amount :type Integer))
  (bind ((`Type_11_A385B47849A45CE53C8EF9BFBE7210D4` _type) (`Amount_49_D1E29AF04498C178B74986AAD5610193` _amount) (`ID_50_BA06E0BD4E97D16461377CB9BF36CE2D` _id)) (break `/Game/MMO/Core/Inventory/S_Item_Info` (`self.ItemInfo`)))
  (return _type _id _amount))

(fn `UserConstructionScript`
  (`parent.UserConstructionScript`)
  (bind _returnvalue (`|GetDataTableRow` "/Game/MMO/Core/Inventory/DT_ArmorList.DT_ArmorList" (`self.InitialID`))
    (:`then`
      (set `self.ItemInfo` (`.ItemInfo_9_747206B9457C40D5BDF581B82BDB6F08` (break `/Game/MMO/Core/Inventory/S_Armor_Info` _returnvalue))))
    (:`RowNotFound`
      (bind _returnvalue_2 (`|GetDataTableRow` "/Game/MMO/Core/Inventory/DT_PotionList.DT_PotionList" (`self.InitialID`))
        (:`then`
          (set `self.ItemInfo` (`.ItemInfo_14_7E8F48144F0F01654500E084A85436C5` (break `/Game/MMO/Core/Inventory/S_Potion_Info` _returnvalue_2))))
        (:`RowNotFound`
          (bind _returnvalue_3 (`|GetDataTableRow` "/Game/MMO/Core/Inventory/DT_WeaponList.DT_WeaponList" (`self.InitialID`))
            (:`then`
              (set `self.ItemInfo` (`.ItemInfo_9_747206B9457C40D5BDF581B82BDB6F08` (break `/Game/MMO/Core/Inventory/S_Weapon_Info` _returnvalue_3)))))))))
  (`StaticMeshComponent.SetStaticMesh` (`self.StaticMesh`) (`.StaticMesh_55_DD99137048858773BCC1349BF67B1BCE` (break `/Game/MMO/Core/Inventory/S_Item_Info` (`self.ItemInfo`)))))