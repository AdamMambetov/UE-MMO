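; Base shield Blueprint for the MMO inventory that handles blocking and contact hits for its owning actor.
; Block and BlockEnd toggle query collision on BlockCollision, and that collision state doubles as the blocking flag.
; Damage the shield receives is forwarded to the owner, cut to a token amount while blocking.
; Overlapping another damageable actor during a specific AC_Attack battle state deals token damage and drops the block.
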(event `self.ReceiveAnyDamage`
  (params (Damage :type "Float (single-precision)") (DamageType :type "DamageType Object Reference") (InstigatedBy :type "Controller Object Reference") (DamageCauser :type "Actor Object Reference"))
  (`GameplayStatics.ApplyDamage` (`self.GetOwner`) (select `bool` (`PrimitiveComponent.K2_IsCollisionEnabled` (`self.BlockCollision`)) :`false` Damage :`true` 1.0) InstigatedBy DamageCauser (`GameplayStatics.GetObjectClass` DamageType)))

(event `self.BlockCollision.OnComponentBeginOverlap`
  (params (OverlappedComponent :type "PrimitiveComponent Object Reference") (OtherActor :type "Actor Object Reference") (OtherComp :type "PrimitiveComponent Object Reference") (OtherBodyIndex :type Integer) (bFromSweep :type Boolean) (SweepResult :type "HitResult Structure (by ref)"))
  (if (and (`Actor.bCanBeDamaged` OtherActor) (!= OtherActor (`self.GetOwner`)) (`|EnumEquality` (`/Game/MMO/Core/BaseCharacter/AC_Attack.BattleState` (`self.GetComponentByClass` (`self.GetOwner`) "/Game/MMO/Core/BaseCharacter/AC_Attack.AC_Attack_C")) "NewEnumerator5"))
    (`GameplayStatics.ApplyDamage` OtherActor 1.0 null self)
    (`self.BlockEnd`)))

(fn `Block`
  (`PrimitiveComponent.SetCollisionEnabled` (`self.BlockCollision`) "QueryOnly"))

(fn `BlockEnd`
  (`PrimitiveComponent.SetCollisionEnabled` (`self.BlockCollision`) "NoCollision"))

(fn `UserConstructionScript`
  (`parent.UserConstructionScript`))