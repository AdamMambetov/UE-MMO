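; BP_Base_Armor is the base Blueprint for an armor item in the inventory system, represented by a static mesh.
; Its construction script looks up InitialID in DT_ArmorList, builds ArmorInfo from that row with InitialAmount as the amount, and applies the row's mesh.
; GetItemInfo exposes the stored item's type, ID and amount.
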(fn `GetItemInfo`
  (returns (Type :type "/Game/MMO/Core/Inventory/E_ItemType Enum") (ID :type Name) (Amount :type Integer))
  (bind ((`Type_11_A385B47849A45CE53C8EF9BFBE7210D4` _type) (`Amount_49_D1E29AF04498C178B74986AAD5610193` _amount) (`ID_50_BA06E0BD4E97D16461377CB9BF36CE2D` _id)) (break `/Game/MMO/Core/Inventory/S_Item_Info` (`.ItemInfo_9_747206B9457C40D5BDF581B82BDB6F08` (break `/Game/MMO/Core/Inventory/S_Armor_Info` (`self.ArmorInfo`)))))
  (return _type _id _amount))

(fn `UserConstructionScript`
  (`parent.UserConstructionScript`)
  (bind _returnvalue (`|GetDataTableRow` "/Game/MMO/Core/Inventory/DT_ArmorList.DT_ArmorList" (`self.InitialID`))
    (:`then`
      (bind (_iteminfo _chunk _armor) (break `/Game/MMO/Core/Inventory/S_Armor_Info` _returnvalue))
      (bind _structout (setmembers `/Game/MMO/Core/Inventory/S_Item_Info` :`StructRef` _iteminfo :`Amount` (`self.InitialAmount`)))
      (bind _output_get (set `self.ArmorInfo` (make `/Game/MMO/Core/Inventory/S_Armor_Info` _structout _chunk _armor)))
      (`StaticMeshComponent.SetStaticMesh` (`self.StaticMesh`) (`.StaticMesh_55_DD99137048858773BCC1349BF67B1BCE` (break `/Game/MMO/Core/Inventory/S_Item_Info` (`.ItemInfo_9_747206B9457C40D5BDF581B82BDB6F08` (break `/Game/MMO/Core/Inventory/S_Armor_Info` _output_get))))))))