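; Actor component for the main character that stores health, stamina and magic stats and exposes them through getters, with setters for current and max health.
; While regen is enabled, Tick applies a delta-time-scaled stamina rate, capped between zero and the maximum.
; SetStaminaRegen changes that rate, so a negative value drains stamina until it hits zero, where the rate resets to a positive default.
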(event `self.ReceiveTick`
  (params (DeltaSeconds :type "Float (single-precision)"))
  ;[1 1 1] Regen
  (if (`self.RegenEnabled`)
    (`self.StaminaRegen`)))

(event `self.ReceiveBeginPlay`
  ;[1 1 1] Default init
)

(fn `GetCurrentHealth`
  (returns (ReturnValue :type "Float (double-precision)"))
  (return (`self.CurrentHealth`)))

(fn `GetCurrentMagic`
  (returns (ReturnValue :type "Float (double-precision)"))
  (return (`self.CurrentMagic`)))

(fn `GetCurrentStamina`
  (returns (ReturnValue :type "Float (double-precision)"))
  (return (`self.CurrentStamina`)))

(fn `GetMaxHealth`
  (returns (ReturnValue :type "Float (double-precision)"))
  (return (`self.MaxHealth`)))

(fn `GetMaxMagic`
  (returns (ReturnValue :type "Float (double-precision)"))
  (return (`self.MaxMagic`)))

(fn `GetMaxStamina`
  (returns (ReturnValue :type "Float (double-precision)"))
  (return (`self.MaxStamina`)))

(fn `SetCurrentHealth`
  (params (Value :type "Float (double-precision)"))
  (returns (Output_Get :type "Float (double-precision)"))
  (bind _output_get (set `self.CurrentHealth` Value))
  (return _output_get))

(fn `SetMaxHealth`
  (params (Value :type "Float (double-precision)"))
  (returns (Output_Get :type "Float (double-precision)"))
  (bind _output_get (set `self.MaxHealth` Value))
  (return _output_get))

(fn `SetStaminaRegen`
  (params (Value :type "Float (double-precision)"))
  (set `self.StaminaRegenVal` Value))

(fn `StaminaRegen`
  (bind _returnvalue (+ (`self.CurrentStamina`) (* (`self.StaminaRegenVal`) (`GameplayStatics.GetWorldDeltaSeconds`))))
  (`/Engine/EditorBlueprintResources/StandardMacros.CompareFloat` (+ (`self.CurrentStamina`) (* (`self.StaminaRegenVal`) (`GameplayStatics.GetWorldDeltaSeconds`))) (`self.MaxStamina`)
    (:`>`
      (set `self.CurrentStamina` (`self.MaxStamina`) :!label _label))
    (:`==`
      (goto _label))
    (:`<`
      (if (<= _returnvalue 0.0)
        (set `self.CurrentStamina` 0.0)
        (set `self.StaminaRegenVal` 1.0)
        (else
          (set `self.CurrentStamina` _returnvalue))))))