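; AI controller for an NPC that patrols until it perceives a target, then switches to attacking.
; It runs the patrol tree on BeginPlay, and successful sight or hearing stimuli store the actor in the "player" blackboard key and start BT_AttackByFeeling.
; Other perception updates clear that key and resume patrol.
; Every Tick copies the main character's combo-attack state into the "PlayerAttack" key.
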(event `self.ReceiveBeginPlay`
  (bind _asbp_main_char (cast `/Game/MMO/Core/MainCharacter/BP_MainChar` (`GameplayStatics.GetPlayerCharacter` 0)))
  (set `self.As BP Main Char` _asbp_main_char)
  (`self.RunBehaviorTree` "/Game/MMO/ai/BT_patrol.BT_patrol"))

(event `CustomEvent_0`
  (if (`BlackboardComponent.GetValueAsBool` (`self.Blackboard`) (`KismetStringLibrary.Conv_StringToName` "sec"))
    (`self.RunBehaviorTree` "/Game/MMO/ai/BT_Refresh.BT_Refresh")
    (`self.RunBehaviorTree` "/Game/MMO/ai/BT_AttackByFeeling.BT_AttackByFeeling")))

(event `self.AIPerception.OnTargetPerceptionUpdated`
  (params (Actor :type "Actor Object Reference") (Stimulus :type "AIStimulus Structure"))
  (bind (_age _expirationage _strength _stimuluslocation _receiverlocation _tag _bsuccessfullysensed) (break `AIStimulus` Stimulus))
  (bind _returnvalue (`KismetStringLibrary.Conv_StringToName` "player"))
  (bind _returnvalue_2 (`KismetStringLibrary.Conv_StringToName` "player"))
  (bind _blackboard (`self.Blackboard`))
  (bind _blackboard_2 (`self.Blackboard`))
  (bind _returnvalue_3 (`AIPerceptionSystem.GetSenseClassForStimulus` Stimulus))
  (bind _returnvalue_4 (`KismetSystemLibrary.GetClassDisplayName` _returnvalue_3))
  (if (and _bsuccessfullysensed (`KismetStringLibrary.EqualEqual_StrStr` _returnvalue_4 "AISense_Sight"))
    (`BlackboardComponent.SetValueAsObject` _blackboard _returnvalue Actor)
    (`self.RunBehaviorTree` "/Game/MMO/ai/BT_AttackByFeeling.BT_AttackByFeeling")
    (else
      (`BlackboardComponent.ClearValue` _blackboard _returnvalue)
      (if (and (`KismetStringLibrary.EqualEqual_StrStr` _returnvalue_4 "AISense_Hearing") _bsuccessfullysensed)
        (`BlackboardComponent.SetValueAsObject` _blackboard_2 _returnvalue_2 Actor)
        (`self.RunBehaviorTree` "/Game/MMO/ai/BT_AttackByFeeling.BT_AttackByFeeling")
        (else
          (`BlackboardComponent.ClearValue` _blackboard_2 _returnvalue_2)
          (`self.RunBehaviorTree` "/Game/MMO/ai/BT_patrol.BT_patrol"))))))

(event `self.ReceiveTick`
  (params (DeltaSeconds :type "Float (single-precision)"))
  (`BlackboardComponent.SetValueAsBool` (`self.Blackboard`) (`KismetStringLibrary.Conv_StringToName` "PlayerAttack") (`/Game/MMO/Core/MainCharacter/BP_MainChar.GetComboAttack` (`self.As BP Main Char`))))

(event `CustomEvent_1`)

(fn `UserConstructionScript`)