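; AI-controlled melee NPC that extends a parent combat character with target sensing, attack and block actions.
; Each tick a forward box trace for pawns sets the AC_first_ncp controller's Overlaped blackboard key, with a DoOnce refreshing the controller once when the trace clears.
; Attack triggers the combo when conditions allow, weapon overlap deals damage then disables its collision, and blocking freezes movement until released.
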(event `self.ReceiveTick`
  (params (DeltaSeconds :type "Float (single-precision)"))
  (bind _capsulecomponent (`self.CapsuleComponent`))
  (bind _returnvalue (`SceneComponent.K2_GetComponentLocation` _capsulecomponent))
  (`parent.ReceiveTick` DeltaSeconds)
  (bind (_outhit _returnvalue_2) (`KismetSystemLibrary.BoxTraceSingleForObjects` _returnvalue (+ _returnvalue (* (`SceneComponent.GetForwardVector` _capsulecomponent) 100.0)) (32.0 50.0 400.0) (struct) (`|MakeArray` "ObjectTypeQuery3" :!type "EObjectTypeQuery Enum")))
  (if _returnvalue_2
    (bind _asac_first_ncp (cast `/Game/MMO/ai/AC_first_ncp` (`self.GetController`)))
    (`BlackboardComponent.SetValueAsBool` (`AIController.Blackboard` _asac_first_ncp) (`KismetStringLibrary.Conv_StringToName` "Overlaped") true)
    (goto _label :!via `Reset`)
    (else
      (bind _asac_first_ncp_2 (cast `/Game/MMO/ai/AC_first_ncp` (`self.GetController`)))
      (`BlackboardComponent.SetValueAsBool` (`AIController.Blackboard` _asac_first_ncp_2) (`KismetStringLibrary.Conv_StringToName` "Overlaped") false)
      (`/Engine/EditorBlueprintResources/StandardMacros.DoOnce` false :!label _label
        (:`Completed`
          (bind _asac_first_ncp_3 (cast `/Game/MMO/ai/AC_first_ncp` (`self.GetController`)))
          (`/Game/MMO/ai/AC_first_ncp.Refresh` _asac_first_ncp_3))))))

(event `Attack`
  (if (`self.ComboAttackConditions`)
    (`self.ComboAttack`)))

(event `self.WeaponCollision.OnComponentBeginOverlap`
  (params (OverlappedComponent :type "PrimitiveComponent Object Reference") (OtherActor :type "Actor Object Reference") (OtherComp :type "PrimitiveComponent Object Reference") (OtherBodyIndex :type Integer) (bFromSweep :type Boolean) (SweepResult :type "HitResult Structure (by ref)"))
  (if (!= OtherActor self)
    (`GameplayStatics.ApplyDamage` OtherActor 2.0)
    (`PrimitiveComponent.SetCollisionEnabled` (`self.WeaponCollision`) "NoCollision")))

(event `CustomBlock`
  (`self.SetBlock` true)
  (`CharacterMovementComponent.DisableMovement` (`self.CharacterMovement`)))

(event `CustomUnBlock`
  (`self.SetBlock` false)
  (`CharacterMovementComponent.SetMovementMode` (`self.CharacterMovement`) "MOVE_Walking" 0))

(fn `UserConstructionScript`
  (`parent.UserConstructionScript`))