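; AI-controlled child character that adds combat actions and detection of the main character.
; Attack runs a combo attack when its conditions pass, while custom block and unblock events toggle blocking and disable or restore walking.
; An overlap component identifies BP_MainCharacter by display name and sets the AC_first_ncp controller's "Overlaped" blackboard flag.
; Ending the overlap clears the flag and calls CustomEvent0 on the controller reference from the begin-overlap cast.
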(event `Attack`
  (if (`self.ComboAttackConditions`)
    (`self.ComboAttack`)))

(event `CustomBlock`
  (`self.SetBlock` true)
  (`CharacterMovementComponent.DisableMovement` (`self.CharacterMovement`)))

(event `CustomUnBlock`
  (`self.SetBlock` false)
  (`CharacterMovementComponent.SetMovementMode` (`self.CharacterMovement`) "MOVE_Walking" 0))

(event `self.  .OnComponentBeginOverlap`
  (params (OverlappedComponent :type "PrimitiveComponent Object Reference") (OtherActor :type "Actor Object Reference") (OtherComp :type "PrimitiveComponent Object Reference") (OtherBodyIndex :type Integer) (bFromSweep :type Boolean) (SweepResult :type "HitResult Structure (by ref)"))
  (if (`KismetStringLibrary.EqualEqual_StrStr` (`KismetSystemLibrary.GetDisplayName` OtherActor) "BP_MainCharacter")
    (bind _asac_first_ncp (cast `/Game/MMO/ai/AC_first_ncp` (`self.GetController`)))
    (`BlackboardComponent.SetValueAsBool` (`AIController.Blackboard` _asac_first_ncp) (`KismetStringLibrary.Conv_StringToName` "Overlaped") true)))

(event `self.  .OnComponentEndOverlap`
  (params (OverlappedComponent :type "PrimitiveComponent Object Reference") (OtherActor :type "Actor Object Reference") (OtherComp :type "PrimitiveComponent Object Reference") (OtherBodyIndex :type Integer))
  (if (`KismetStringLibrary.EqualEqual_StrStr` (`KismetSystemLibrary.GetDisplayName` OtherActor) "BP_MainCharacter")
    (bind _asac_first_ncp (cast `/Game/MMO/ai/AC_first_ncp` (`self.GetController`)))
    (`BlackboardComponent.SetValueAsBool` (`AIController.Blackboard` _asac_first_ncp) (`KismetStringLibrary.Conv_StringToName` "Overlaped") false)
    (`/Game/MMO/ai/AC_first_ncp.CustomEvent_0` (stale `self.  .OnComponentBeginOverlap` _asac_first_ncp))))

(fn `UserConstructionScript`
  (`parent.UserConstructionScript`))