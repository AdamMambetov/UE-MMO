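; Bandit NPC that equips a sword and shield, then fights actors it hears or sees.
; Hearing and sight events from its AI controller branch on the actor's first tag to claim a free AI slot on that actor, start combat, or both.
; Combat stores the target in the Blackboard and runs the fight tree when overlapped and in position.
; When not overlapped, it rolls a random action and runs a move tree chosen by target interface.
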(event `self.ReceiveBeginPlay`
  ;[1 1 1] Begin Play
  (`parent.ReceiveBeginPlay`)
  (bind _asaic_base_npc (cast `/Game/MMO/ai/AIC_BaseNpc` (`self.GetController`)))
  (bind _output_get (set `self.As AIC Base Npc` _asaic_base_npc))
  (add `/Game/MMO/ai/AIC_BaseNpc.Hearing_Update` _output_get (`|CreateDelegate` :!event `Hearing_Update`))
  (add `/Game/MMO/ai/AIC_BaseNpc.Sight_Update` _output_get (`|CreateDelegate` :!event `Sight_Update`))
  (set `self.AiController` (`AIBlueprintHelperLibrary.GetAIController` self))
  (set `self.Base Damage` 1.0)
  (`BlackboardComponent.SetValueAsBool` (`AIController.Blackboard` (`self.As AIC Base Npc`)) (`KismetStringLibrary.Conv_StringToName` "FinishPos") true)
  (`self.EquipmentSetup`))

(event `Hearing_Update`
  (params (Actor :type "Actor Object Reference"))
  ;[1 1 1] Hearing Update
  (set `self.Actor` Actor)
  (switch `name` (`|GetArrayItem` (`Actor.Tags` (`self.Actor`)))
    (:`Default`
      (`self.FightScene`))
    (:`Bandit`
      (`self.SetAiSlot`))))

(event `Sight_Update`
  (params (Actor :type "Actor Object Reference"))
  ;[1 1 1] Sight Update
  (set `self.Actor` Actor)
  (switch `name` (`|GetArrayItem` (`Actor.Tags` (`self.Actor`)))
    (:`Default`
      (`|ExecutionSequence`
        (:`then_0`
          (`self.SetAiSlot`))
        (:`then_1`
          (`self.FightScene`))))))

(fn `EquipmentSetup`
  (bind _inventory (`self.Inventory`)
    (:`then`
      (bind _returnvalue (`/Game/MMO/Core/Inventory/AC_Inventory.AddItem` _inventory "NewEnumerator0" "sword" 1))
      (if _returnvalue
        (`/Game/MMO/Core/Inventory/AC_Inventory.UseItemAtIndex` (`self.Inventory`) 0)
        (bind _returnvalue_2 (`/Game/MMO/Core/Inventory/AC_Inventory.AddItem` (`self.Inventory`) "NewEnumerator1" "shield" 1))
        (if _returnvalue_2
          (`/Game/MMO/Core/Inventory/AC_Inventory.UseItemAtIndex` (`self.Inventory`) 1))))
    (:`else`)))

(fn `FightScene`
  (`/Engine/EditorBlueprintResources/StandardMacros.IsValid` (`BlackboardComponent.GetValueAsObject` (`AIController.Blackboard` (`self.As AIC Base Npc`)) (`KismetStringLibrary.Conv_StringToName` "player"))
    (:`Is Valid`
      _)
    (:`Is Not Valid`
      (`BlackboardComponent.SetValueAsObject` (`AIController.Blackboard` (`self.As AIC Base Npc`)) (`KismetStringLibrary.Conv_StringToName` "player") (`self.Actor`))))
  (if (`BlackboardComponent.GetValueAsBool` (`AIController.Blackboard` (`self.As AIC Base Npc`)) (`KismetStringLibrary.Conv_StringToName` "Overlaped"))
    (if (`BlackboardComponent.GetValueAsBool` (`AIController.Blackboard` (`self.As AIC Base Npc`)) (`KismetStringLibrary.Conv_StringToName` "FinishPos"))
      (set `self.EMovementState` "NewEnumerator1")
      (`AIController.RunBehaviorTree` (`self.AiController`) "/Game/MMO/ai/BehaviorTree/BT_Fight.BT_Fight"))
    (else
      (`self.Roll_Action`)
      (set `self.EMovementState` "NewEnumerator2")
      (if (`KismetSystemLibrary.DoesImplementInterface` (`self.Actor`) "/Game/MMO/Characters/MainCharacter/BPI_MainCharacter.BPI_MainCharacter_C")
        (`AIController.RunBehaviorTree` (`self.AiController`) "/Game/MMO/ai/BehaviorTree/BT_MoveToFightPos.BT_MoveToFightPos")
        (else
          (`AIController.RunBehaviorTree` (`self.AiController`) "/Game/MMO/ai/BehaviorTree/MoveTo.MoveTo"))))))

(fn `Roll_Action`
  (`BlackboardComponent.SetValueAsInt` (`AIBlueprintHelperLibrary.GetBlackboard` (`AIBlueprintHelperLibrary.GetAIController` self)) (`KismetStringLibrary.Conv_StringToName` "Action") (`KismetMathLibrary.RandomInteger` 2)))

(fn `SetAiSlot`
  (`/Engine/EditorBlueprintResources/StandardMacros.DoOnce` false
    (:`Completed`
      (bind _returnarray (message `/Game/MMO/Core/BaseCharacter/BPI_BaseCharacter.GetAiSlotsInfo` (`self.Actor`)))
      (for _array_element _returnarray
        (bind (_postion _location _bplaced) (break `/Game/MMO/Core/BaseCharacter/S_AiSlotInfo` _array_element))
        (if (not _bplaced)
          (message `/Game/MMO/Core/BaseCharacter/BPI_BaseCharacter.SetAiSlotPlaced` (`self.Actor`) true _postion)
          (`BlackboardComponent.SetValueAsEnum` (`AIController.Blackboard` (`self.As AIC Base Npc`)) (`KismetStringLibrary.Conv_StringToName` "Aislot") _postion)
          (break))))))

(fn `UserConstructionScript`
  (`parent.UserConstructionScript`))