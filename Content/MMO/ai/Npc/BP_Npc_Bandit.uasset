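; Bandit NPC Blueprint that switches to combat behavior when it hears or sees an actor.
; On BeginPlay it casts its controller to AIC_BaseNpc and binds handlers to that controller's hearing and sight updates.
; Both handlers switch on the actor's first tag, but only a default branch exists, which stores the actor in the "player" Blackboard key and runs BT_Fight.
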(event `self.ReceiveBeginPlay`
  (`parent.ReceiveBeginPlay`)
  (bind _asaic_base_npc (cast `/Game/MMO/ai/AIC_BaseNpc` (`self.GetController`)))
  (bind _output_get (set `self.As AIC Base Npc` _asaic_base_npc))
  (add `/Game/MMO/ai/AIC_BaseNpc.Hearing_Update` _output_get (delegate `Hearing_Update`))
  (add `/Game/MMO/ai/AIC_BaseNpc.Sight_Update` _output_get (delegate `Sight_Update`)))

(event `Hearing_Update`
  (params (Actor :type "Actor Object Reference"))
  (switch `name` (`|GetArrayItem` (`Actor.Tags` Actor))
    (:`Default`
      (`BlackboardComponent.SetValueAsObject` (`AIController.Blackboard` (`self.As AIC Base Npc`)) (`KismetStringLibrary.Conv_StringToName` "player") Actor)
      (`AIController.RunBehaviorTree` (`self.As AIC Base Npc`) "/Game/MMO/ai/BT_Fight.BT_Fight"))))

(event `Sight_Update`
  (params (Actor :type "Actor Object Reference"))
  (switch `name` (`|GetArrayItem` (`Actor.Tags` Actor))
    (:`Default`
      (`BlackboardComponent.SetValueAsObject` (`AIController.Blackboard` (`self.As AIC Base Npc`)) (`KismetStringLibrary.Conv_StringToName` "player") Actor)
      (`AIController.RunBehaviorTree` (`self.As AIC Base Npc`) "/Game/MMO/ai/BT_Fight.BT_Fight"))))

(fn `UserConstructionScript`
  (`parent.UserConstructionScript`))