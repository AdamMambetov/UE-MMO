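; Base NPC Blueprint that detects pawns of a different group nearby and reports them to its AI Blackboard.
; Each Tick it box-traces along the capsule's forward axis, comparing first actor tags to set "Overlaped", with the last hit winning.
; The trace's front reach adds Blackboard "fault_50", whose random range is fixed at one value.
; Battle mode turns on orient-to-movement, while Block and UnBlock are empty, their movement-toggle logic left disconnected.
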(event `self.ReceiveBeginPlay`
  (`parent.ReceiveBeginPlay`)
  (`BlackboardComponent.SetValueAsFloat` (`AIBlueprintHelperLibrary.GetBlackboard` (`self.GetController`)) (`KismetStringLibrary.Conv_StringToName` "fault_50") (`KismetMathLibrary.RandomFloatInRange` 1.0 1.0)))

(event `self.ReceiveTick`
  (params (DeltaSeconds :type "Float (single-precision)"))
  (bind _returnvalue (`KismetStringLibrary.Conv_StringToName` "Overlaped"))
  (bind _capsulecomponent (`self.CapsuleComponent`))
  (bind _returnvalue_2 (`AIBlueprintHelperLibrary.GetBlackboard` (`self.GetController`)))
  (bind _returnvalue_3 (`SceneComponent.K2_GetComponentLocation` _capsulecomponent))
  (bind _returnvalue_4 (`SceneComponent.GetForwardVector` _capsulecomponent))
  ;[1 1 1] BoxTrace
  (`parent.ReceiveTick` DeltaSeconds)
  (bind (_outhits _returnvalue_5) (`KismetSystemLibrary.BoxTraceMultiForObjects` (+ (* _returnvalue_4 -300.0) _returnvalue_3) (+ _returnvalue_3 (* _returnvalue_4 (+ 300.0 (`BlackboardComponent.GetValueAsFloat` (`AIBlueprintHelperLibrary.GetBlackboard` (`self.GetController`)) (`KismetStringLibrary.Conv_StringToName` "fault_50"))))) (0.0 300.0 300.0) (`self.K2_GetActorRotation`) (`|MakeArray` "ObjectTypeQuery3" :!type "EObjectTypeQuery Enum") true))
  (if _returnvalue_5
    (for _array_element _outhits
      (bind (_bblockinghit _binitialoverlap _time _distance _location _impactpoint _normal _impactnormal _physmat _hitactor) (`GameplayStatics.BreakHitResult` _array_element))
      (bind _returnvalue_6 (!= (`|GetArrayItem` (`Actor.Tags` _hitactor)) (`|GetArrayItem` (`self.Tags`))))
      (if _returnvalue_6
        (if (or (== _hitactor (`BlackboardComponent.GetValueAsObject` (`AIBlueprintHelperLibrary.GetBlackboard` (`self.GetController`)) (`KismetStringLibrary.Conv_StringToName` "player"))) _returnvalue_6)
          (`BlackboardComponent.SetValueAsBool` _returnvalue_2 _returnvalue true)
          (else
            (`BlackboardComponent.SetValueAsBool` _returnvalue_2 _returnvalue false :!label _label)
            (`BlackboardComponent.SetValueAsFloat` (`AIBlueprintHelperLibrary.GetBlackboard` (`self.GetController`)) (`KismetStringLibrary.Conv_StringToName` "fault_50") (`KismetMathLibrary.RandomFloatInRange` 1.0 1.0))))
        (else
          (goto _label))))
    (else
      (goto _label))))

(event `/Game/MMO/Core/BaseCharacter/BPI_BaseCharacter.EnableBattleMode`
  (`parent.EnableBattleMode`)
  (set `CharacterMovementComponent.bOrientRotationToMovement` true (`self.CharacterMovement`)))

(event `Block`
  ;[1 1 1] Block
)

(event `UnBlock`
  ;[1 1 1] Block
)

(fn `UserConstructionScript`
  (`parent.UserConstructionScript`))